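; Trigger volume that changes the third-person character's camera view while the character overlaps its box.
; With ChangeToNewCamera set, it blends the view target to itself, then matches control rotation to its camera, and blends back on exit.
; Otherwise, timelines lerp the character's camera boom length and rotation to the new values and restore the cached originals on exit.
; Camera-look lock logic is present but unconnected.
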(event OnComponentBeginOverlap(Box)
  (params (OverlappedComponent :type Primitive%20Component%20Object%20Reference) (OtherActor :type Actor%20Object%20Reference) (OtherComp :type Primitive%20Component%20Object%20Reference) (OtherBodyIndex :type Integer) (bFromSweep :type Boolean) (SweepResult :type Hit%20Result%20Structure%20%28by%20ref%29))
  (bind _asbp_third_person_character (Utilities|Casting|CastToBP_ThirdPersonCharacter OtherActor))
  (bind _output_get (Variables|Default|SetCharacterRef _asbp_third_person_character))
  (if (Variables|Default|GetChangeToNewCamera)
    ;[0.15 0.15 0.15 0.5] Switch To Static Camera
    (Game|Player|SetViewTargetwithBlend (Game|GetPlayerController 0) self 1.0 "VTBlend_Linear" 0.0 false)
    (Utilities|FlowControl|Delay 1.0)
    (Pawn|SetControlRotation (Game|GetPlayerController 0) (Transformation|GetWorldRotation (Variables|Default|GetCamera)))
    (else
      ;[0.15 0.15 0.15 0.5] Change Camera Boom Rotation and Location
      (Variables|Default|SetOriginalRotation (Variables|/Script/Engine.SceneComponent|GetRelativeRotation (Variables|/Script/Pravda_Concept25.Pravda_Concept25Character|GetCameraBoom _output_get)))
      (Variables|Default|SetOriginalArmLength (Variables|/Script/Engine.SpringArmComponent|GetTargetArmLength (Variables|/Script/Pravda_Concept25.Pravda_Concept25Character|GetCameraBoom _output_get)))
      (bind _newtrack_0 (Timeline|Timeline PlayFromStart)
        (:Update
          (Variables|/Script/Engine.SpringArmComponent|SetTargetArmLength (Variables|/Script/Pravda_Concept25.Pravda_Concept25Character|GetCameraBoom (Variables|Default|GetCharacterRef)) (Math|Float|Lerp (Variables|Default|GetOriginalArmLength) (Variables|Default|GetNewViewArmLength) _newtrack_0))
          (Transformation|SetRelativeRotation (Variables|/Script/Pravda_Concept25.Pravda_Concept25Character|GetCameraBoom (Variables|Default|GetCharacterRef)) (Math|Rotator|Lerp(Rotator) (Variables|Default|GetOriginalRotation) (Variables|Default|GetNewViewRotation) _newtrack_0) false false))))))

(event OnComponentEndOverlap(Box)
  (params (OverlappedComponent :type Primitive%20Component%20Object%20Reference) (OtherActor :type Actor%20Object%20Reference) (OtherComp :type Primitive%20Component%20Object%20Reference) (OtherBodyIndex :type Integer))
  (bind _characterref (Variables|Default|GetCharacterRef))
  (bind _cameraboom (Variables|/Script/Pravda_Concept25.Pravda_Concept25Character|GetCameraBoom _characterref))
  (Utilities|Casting|CastToBP_ThirdPersonCharacter OtherActor)
  (if (Variables|Default|GetChangeToNewCamera)
    ;[0.15 0.15 0.15 0.5] Revert To Player Camera
    (Game|Player|SetViewTargetwithBlend (Game|GetPlayerController 0) (Variables|Default|GetCharacterRef) 1.0 "VTBlend_Linear" 0.0 false)
    (else
      ;[0.15 0.15 0.15 0.5] Revert To Original Position
      (bind _newtrack_0 (Timeline|Timeline_0 PlayFromStart)
        (:Update
          (Variables|/Script/Engine.SpringArmComponent|SetTargetArmLength _cameraboom (Math|Float|Lerp (Variables|Default|GetNewViewArmLength) (Variables|Default|GetOriginalArmLength) _newtrack_0))
          (Transformation|SetRelativeRotation _cameraboom (Math|Rotator|Lerp(Rotator) (Variables|Default|GetNewViewRotation) (Variables|Default|GetOriginalRotation) _newtrack_0) false false))))))

(fn ConstructionScript)