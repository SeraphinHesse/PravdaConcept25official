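; Photo-mode minigame actor that shows an adjustable vision cone aimed at the point under the cursor.
; StartPhotoMode hides the cursor, starts a self-rescheduling aim timer and applies a dynamic cone material to a decal or plane via UseDecal, though both branches show only the decal.
; Holding E or Q runs timelines sweeping cone angle or decal radius.
; Left click restores character camera and walking, then destroys the actor without capturing anything.
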(event Custom|StartPhotoMode
  (bind _outerradius (Variables|VisionArea|GetOuterRadius))
  (bind _outerradius_2 (Variables|VisionArea|GetOuterRadius))
  (bind _returnvalue (/ _outerradius_2 256.0))
  (bind _returnvalue_2 (/ _outerradius 5e+01))
  (Variables|/Script/Engine.PlayerController|SetbShowMouseCursor (Game|GetPlayerController 0) false)
  (CallFunction|AimPhoto)
  (Input|EnableInput (Game|GetPlayerController 0))
  (if (Variables|VisionArea|GetbUseDecal)
    ;[0.15 0.15 0.15 0.5] SetVisionAreaDecal
    (Rendering|SetVisibility (Variables|Default|GetPlane) false false)
    (Rendering|SetVisibility (Variables|Default|GetDecal) true false)
    (bind _returnvalue_3 (Rendering|Material|CreateDynamicMaterialInstance "/Game/Assets/Materials/M_CameraMinigameDecal.M_CameraMinigameDecal" "None" "None" :!class /Script/Engine.KismetMaterialLibrary))
    (bind _output_get (Variables|Default|SetDMIDecal _returnvalue_3))
    (Rendering|Components|Decal|SetDecalMaterial (Variables|Default|GetDecal) _output_get)
    (Rendering|Material|SetScalarParameterValue _output_get "HalfAngle" (Variables|VisionArea|GetHalfAngle) :!class /Script/Engine.MaterialInstanceDynamic)
    (Transformation|SetRelativeScale3D (Variables|Default|GetDecal) (Math|Vector|MakeVector 1e+01 _returnvalue _returnvalue))
    (Rendering|Material|SetScalarParameterValue (Variables|Default|GetDMIDecal) "InternalRadius" (* (/ (Variables|VisionArea|GetInnerRadius) (Variables|VisionArea|GetOuterRadius)) 0.5) :!class /Script/Engine.MaterialInstanceDynamic)
    (else
      ;[0.15 0.15 0.15 0.5] ProjectVisionConeOnPlane
      (Rendering|SetVisibility (Variables|Default|GetPlane) false false)
      (Rendering|SetVisibility (Variables|Default|GetDecal) true false)
      (bind _returnvalue_4 (Rendering|Material|CreateDynamicMaterialInstance "/Game/Assets/Materials/M_CameraMinigame.M_CameraMinigame" "None" "None" :!class /Script/Engine.KismetMaterialLibrary))
      (bind _output_get_2 (Variables|Default|SetDMIDecal _returnvalue_4))
      (Rendering|Material|SetMaterial (Variables|Default|GetPlane) 0 _output_get_2)
      (Rendering|Material|SetScalarParameterValue _output_get_2 "HalfAngle" (Variables|VisionArea|GetHalfAngle) :!class /Script/Engine.MaterialInstanceDynamic)
      (Transformation|SetRelativeScale3D (Variables|Default|GetPlane) (Math|Vector|MakeVector _returnvalue_2 _returnvalue_2 1.0))
      (Rendering|Material|SetScalarParameterValue (Variables|Default|GetDMIDecal) "InternalRadius" (* (/ (Variables|VisionArea|GetInnerRadius) (Variables|VisionArea|GetOuterRadius)) 0.5) :!class /Script/Engine.MaterialInstanceDynamic))))

(event Custom|AimPhoto
  (bind _returnvalue (Transformation|GetActorLocation))
  (bind _returnvalue_2 (Game|GetPlayerController 0))
  (bind _hitresult (Game|Player|GetHitResultUnderCursorbyChannel _returnvalue_2 "TraceTypeQuery1" true))
  (bind _location (Collision|BreakHitResult _hitresult))
  ;[1 0.8121 0.2952] Rotate Actor With Mouse
  (bind _returnvalue_3 (Utilities|Time|SetTimerbyEvent (delegate Custom|AimPhoto) 0.01))
  (Variables|Default|SetTimerForAiming _returnvalue_3)
  (Transformation|SetActorRotation (Math|Rotator|FindLookatRotation (Math|Vector|MakeVector (.x _returnvalue) (.y _returnvalue) 0.0) (Math|Vector|MakeVector (.x _location) (.y _location) 0.0))))

(event Input|KeyboardEvents|Q
  (params (Key :type Key%20Structure :default "None"))
  ;[0.15 0.15 0.15 0.5] ChangeVisionRadius
  (:Pressed
    (Components|Timeline|SetPlayRate (Variables|Default|GetTimeline) (Variables|Default|GetNew%20Rate))
    (bind _newtrack_0 (Timeline|Timeline_0 PlayFromStart)
      (:Update
        (Transformation|SetRelativeScale3D (Variables|Default|GetDecal) (Math|Vector|MakeVector 1e+01 (/ (Math|Float|Lerp 1e+02 1e+03 _newtrack_0) 256.0) (/ (Math|Float|Lerp 1e+02 1e+03 _newtrack_0) 256.0))))))
  (:Released
    (Timeline|Timeline_0 Stop)))

(event Input|MouseEvents|LeftMouseButton
  (params (Key :type Key%20Structure :default "None"))
  ;[0.15 0.15 0.15 0.5] Make a photo
  (:Pressed
    (bind _returnvalue (Actor|GetActorOfClass "/Game/SC_ThirdPerson/Blueprints/BP_ThirdPersonCharacter.BP_ThirdPersonCharacter_C"))
    (Variables|/Script/Engine.SpringArmComponent|SetbUsePawnControlRotation (Variables|/Script/Pravda_Concept25.Pravda_Concept25Character|GetCameraBoom _returnvalue) true)
    (Pawn|Components|CharacterMovement|SetMovementMode (Variables|/Script/Engine.Character|GetCharacterMovement _returnvalue) "MOVE_Walking" 0)
    (Actor|DestroyActor)))

(event Input|KeyboardEvents|E
  (params (Key :type Key%20Structure :default "None"))
  ;[0.15 0.15 0.15 0.5] ChangeConeAngle
  (:Pressed
    (Components|Timeline|SetPlayRate (Variables|Default|GetTimeline) (Variables|Default|GetNew%20Rate))
    (bind _newtrack_0 (Timeline|Timeline PlayFromStart)
      (:Update
        (Rendering|Material|SetScalarParameterValue (Variables|Default|GetDMIDecal) "HalfAngle" (Math|Float|Lerp 0.0 9e+01 _newtrack_0) :!class /Script/Engine.MaterialInstanceDynamic))))
  (:Released
    (Timeline|Timeline Stop)))

(fn ConstructionScript)